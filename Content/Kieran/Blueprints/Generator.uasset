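; Generator puzzle Blueprint that starts running once it has a Lever item installed and is receiving power from three switches.
; On BeginPlay it registers itself with each switch, and its flicked-switch event sets power only when all three switch puzzles are complete.
; Pressing E while the prompt text is visible installs the Lever from the player's item list.
; Both paths run a completion check that updates the light color, and on success the status text.
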(event Custom|flicked%20switch
  (if (Math|Boolean|ANDBoolean (Variables|/Game/Kieran/Blueprints/InteractableObject.InteractableObject_C|GetpuzzleComplete (Variables|Default|Getswitch1)) (Variables|/Game/Kieran/Blueprints/InteractableObject.InteractableObject_C|GetpuzzleComplete (Variables|Default|Getswitch2)) (Variables|/Game/Kieran/Blueprints/InteractableObject.InteractableObject_C|GetpuzzleComplete (Variables|Default|Getswitch3)))
    (Variables|Default|SetgettingPower true)
    (else
      (Variables|Default|SetgettingPower false)))
  (CallFunction|Checkcomple))

(event Custom|checkcomple
  (if (and (Variables|Default|GetHasLever) (Variables|Default|GetgettingPower))
    (Development|PrintString "Generator On!")
    (Variables|Default|SetpuzzleComplete true)
    (Rendering|Components|TextRender|SetText (Variables|Default|GetTextRender) (Utilities|Text|MakeLiteralText "Running!"))
    (Rendering|Components|Light|SetLightColor (Variables|Default|GetPointLight) (Variables|Default|Geton%20color) true)
    (else
      (Development|PrintString "Won't turn on!")
      (Rendering|Components|Light|SetLightColor (Variables|Default|GetPointLight) (Variables|Default|Getoff%20color) true))))

(event EventBeginPlay
  (|CallParentFunction)
  (Default|GetGEn (Variables|Default|Getswitch1) self)
  (Default|GetGEn (Variables|Default|Getswitch2) self)
  (Default|GetGEn (Variables|Default|Getswitch3) self))

(event Collision|EventActorBeginOverlap
  (params (OtherActor :type Actor%20Object%20Reference))
  (|CallParentFunction OtherActor) ; This node is disabled and will not be called.\nDrag off pins to build functionality.
)

(event EventTick
  (params (DeltaSeconds :type Float%20%28single-precision%29))
  (|CallParentFunction DeltaSeconds)
  (if (and (Variables|Default|GetTextVis) (not (Variables|Default|GetpuzzleComplete)))
    (if (Variables|/Game/ThirdPersonBP/Blueprints/ThirdPersonCharacter.ThirdPersonCharacter_C|GetPressE (Variables|Default|Getplayer))
      (CallFunction|PuzzleFunction))))

(fn ConstructionScript
  (|CallParentFunction))

(fn PuzzleFunction
  (|CallParentFunction)
  (bind _found1 (CallFunction|LookforItem "Lever"))
  (if _found1
    (Variables|Default|SetHasLever true)
    (Rendering|SetVisibility (Variables|Default|Getlever) true false)
    (Utilities|Array|RemoveItem (Variables|/Game/ThirdPersonBP/Blueprints/ThirdPersonCharacter.ThirdPersonCharacter_C|GetItemList (Variables|Default|Getplayer)) "Lever")
    (CallFunction|Checkcomple)))