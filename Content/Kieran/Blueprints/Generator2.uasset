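; Generator2 is a puzzle object, apparently the final one, that completes when the player presses E with the "Gen" item and then ends the level.
; Tick checks inherited prompt and player state, then reveals the generator's components, clears the prompt text and marks the puzzle complete.
; A one-time delayed sequence activates lightning, then swirl effects, each with a camera shake, before opening the EndMenu level.
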(event EventBeginPlay
  (|CallParentFunction)
  (Variables|Default|Setplayer 0)
  (Components|Activation|Deactivate (Variables|/Script/Engine.Actor|GetRootComponent (Variables|Default|GetLightning)))
  (Components|Activation|Deactivate (Variables|/Script/Engine.Actor|GetRootComponent (Variables|Default|GetSwirls))))

(event Collision|EventActorBeginOverlap
  (params (OtherActor :type Actor%20Object%20Reference))
  (|CallParentFunction OtherActor) ; This node is disabled and will not be called.\nDrag off pins to build functionality.
)

(event EventTick
  (params (DeltaSeconds :type Float%20%28single-precision%29))
  (bind _player (Variables|Default|Getplayer))
  (|CallParentFunction DeltaSeconds)
  (if (and (Variables|Default|GetTextVis) (not (Variables|Default|GetpuzzleComplete)))
    (if (Variables|/Game/ThirdPersonBP/Blueprints/ThirdPersonCharacter.ThirdPersonCharacter_C|GetPressE (Variables|Default|Getplayer))
      (bind _found1 (CallFunction|LookforItem "Gen"))
      (if _found1
        (Rendering|SetVisibility (Variables|Default|GetDefaultSceneRoot) true true)
        (Variables|Default|SetpuzzleComplete true)
        (Rendering|Components|TextRender|SetText (Variables|Default|GetTextRender) (Utilities|Text|MakeLiteralText ""))
        (Utilities|FlowControl|DoOnce false
          (:Completed
            (Utilities|FlowControl|Delay 0.2)
            (Components|Activation|Activate (Variables|/Script/Engine.Actor|GetRootComponent (Variables|Default|GetLightning)) false)
            (Variables|Default|SetPlayerRef _player)
            (Camera|PlayWorldCameraShake "/Game/Scripts/Natan/CameraShake.CameraShake_C" (Transformation|GetWorldLocation (Variables|/Game/ThirdPersonBP/Blueprints/ThirdPersonCharacter.ThirdPersonCharacter_C|GetFollowCamera _player)) 0.0 5e+02)
            (Utilities|FlowControl|Delay 2.0)
            (Components|Activation|Activate (Variables|/Script/Engine.Actor|GetRootComponent (Variables|Default|GetSwirls)) false)
            (Camera|PlayWorldCameraShake "/Game/Scripts/Natan/CameraShake_3.CameraShake_3_C" (Transformation|GetWorldLocation (Variables|/Game/ThirdPersonBP/Blueprints/ThirdPersonCharacter.ThirdPersonCharacter_C|GetFollowCamera (Variables|Default|GetPlayerRef))) 0.0 5e+02)
            (Utilities|FlowControl|Delay 3.5)
            (Game|OpenLevel(byName) "EndMenu")))))))

(fn ConstructionScript
  (|CallParentFunction))

(fn PuzzleFunction
  (|CallParentFunction))