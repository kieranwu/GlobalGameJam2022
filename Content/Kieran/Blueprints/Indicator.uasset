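; Indicator actor that shows progress on three linked puzzles (Puzzle1, Puzzle10, Puzzle11) by lighting a point light for each.
; Tick polls each puzzle's PuzzleComplete flag and uses a DoOnce to make the matching light visible.
; When all three are solved it sets its own PuzzleComplete flag, which also stops further checks.
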(event EventBeginPlay)

(event Collision|EventActorBeginOverlap
  (params (OtherActor :type Actor%20Object%20Reference)))

(event EventTick
  (params (DeltaSeconds :type Float%20%28single-precision%29))
  (if (not (Variables|Default|GetpuzzleComplete))
    (Utilities|FlowControl|Sequence
      (:then_0
        (if (Variables|/Game/Kieran/Blueprints/InteractableObject.InteractableObject_C|GetpuzzleComplete (Variables|Default|Getpuzzle1))
          (Utilities|FlowControl|DoOnce false
            (:Completed
              (Rendering|SetVisibility (Variables|Default|GetPointLight) true true)))))
      (:then_1
        (if (Variables|/Game/Kieran/Blueprints/InteractableObject.InteractableObject_C|GetpuzzleComplete (Variables|Default|Getpuzzle1_0))
          (Utilities|FlowControl|DoOnce false
            (:Completed
              (Rendering|SetVisibility (Variables|Default|GetPointLight1) true true)))))
      (:then_2
        (if (Variables|/Game/Kieran/Blueprints/InteractableObject.InteractableObject_C|GetpuzzleComplete (Variables|Default|Getpuzzle1_1))
          (Utilities|FlowControl|DoOnce false
            (:Completed
              (Rendering|SetVisibility (Variables|Default|GetPointLight2) true true)))))
      (:then_3
        (if (Math|Boolean|ANDBoolean (Variables|/Game/Kieran/Blueprints/InteractableObject.InteractableObject_C|GetpuzzleComplete (Variables|Default|Getpuzzle1)) (Variables|/Game/Kieran/Blueprints/InteractableObject.InteractableObject_C|GetpuzzleComplete (Variables|Default|Getpuzzle1_0)) (Variables|/Game/Kieran/Blueprints/InteractableObject.InteractableObject_C|GetpuzzleComplete (Variables|Default|Getpuzzle1_1)))
          (Variables|Default|SetpuzzleComplete true))))))

(fn ConstructionScript)