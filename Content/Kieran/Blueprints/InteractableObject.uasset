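; Base interactable object that highlights itself and shows a text prompt while the player is inside its box trigger.
; Overlap events store or clear the player, toggle the "selected" material parameter and set text visibility.
; While the text shows, Tick rotates it and its backing toward the player's follow camera.
; LookForItem searches the player's item list by name, and PickUpFunction and PuzzleFunction are empty stubs.
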(event OnComponentBeginOverlap(Box)
  (params (OverlappedComponent :type Primitive%20Component%20Object%20Reference) (OtherActor :type Actor%20Object%20Reference) (OtherComp :type Primitive%20Component%20Object%20Reference) (OtherBodyIndex :type Integer) (bFromSweep :type Boolean) (SweepResult :type Hit%20Result%20Structure%20%28by%20ref%29))
  (if (== OtherActor (Game|GetPlayerCharacter 0))
    (bind _asthird_person_character (Utilities|Casting|CastToThirdPersonCharacter OtherActor))
    (Variables|Default|Setplayer _asthird_person_character)
    (Variables|Default|SetTextVis true)
    (Variables|Default|SetParameter%20Value 1.0)
    (Rendering|Material|SetScalarParameterValueonMaterials (Variables|Default|GetBase%20Mesh) "selected" (Variables|Default|GetParameter%20Value))
    (Rendering|SetVisibility (Variables|Default|GetTextBack) (Variables|Default|GetTextVis) true)))

(event OnComponentEndOverlap(Box)
  (params (OverlappedComponent :type Primitive%20Component%20Object%20Reference) (OtherActor :type Actor%20Object%20Reference) (OtherComp :type Primitive%20Component%20Object%20Reference) (OtherBodyIndex :type Integer))
  (if (== OtherActor (Game|GetPlayerCharacter 0))
    (Variables|Default|Setplayer 0)
    (Variables|Default|SetTextVis false)
    (Variables|Default|SetParameter%20Value 0.0)
    (Rendering|Material|SetScalarParameterValueonMaterials (Variables|Default|GetBase%20Mesh) "selected" (Variables|Default|GetParameter%20Value))
    (Rendering|SetVisibility (Variables|Default|GetTextBack) (Variables|Default|GetTextVis) true)))

(event Custom|FacePlayer
  (bind _asthird_person_character (Utilities|Casting|CastToThirdPersonCharacter (Game|GetPlayerCharacter 0)))
  (Transformation|SetWorldRotation (Variables|Default|GetTextBack) (Math|Conversions|RotationFromXVector (Math|Vector|RotateVector (Math|Vector|Normalize (Math|Vector|MakeVector (.x (- (Transformation|GetWorldLocation (Variables|/Game/ThirdPersonBP/Blueprints/ThirdPersonCharacter.ThirdPersonCharacter_C|GetFollowCamera _asthird_person_character)) (Transformation|GetWorldLocation (Variables|Default|GetDefaultSceneRoot)))) (.y (- (Transformation|GetWorldLocation (Variables|/Game/ThirdPersonBP/Blueprints/ThirdPersonCharacter.ThirdPersonCharacter_C|GetFollowCamera _asthird_person_character)) (Transformation|GetWorldLocation (Variables|Default|GetDefaultSceneRoot)))) (.z (- (Transformation|GetWorldLocation (Variables|/Game/ThirdPersonBP/Blueprints/ThirdPersonCharacter.ThirdPersonCharacter_C|GetFollowCamera _asthird_person_character)) (Transformation|GetWorldLocation (Variables|Default|GetDefaultSceneRoot)))))) "0.000000,90.000000,0.000000")) false false)
  (Transformation|SetWorldRotation (Variables|Default|GetTextRender) (Math|Conversions|RotationFromXVector (Math|Vector|RotateVector (Math|Vector|Normalize (Math|Vector|MakeVector (.x (- (Transformation|GetWorldLocation (Variables|/Game/ThirdPersonBP/Blueprints/ThirdPersonCharacter.ThirdPersonCharacter_C|GetFollowCamera _asthird_person_character)) (Transformation|GetWorldLocation (Variables|Default|GetDefaultSceneRoot)))) (.y (- (Transformation|GetWorldLocation (Variables|/Game/ThirdPersonBP/Blueprints/ThirdPersonCharacter.ThirdPersonCharacter_C|GetFollowCamera _asthird_person_character)) (Transformation|GetWorldLocation (Variables|Default|GetDefaultSceneRoot)))) (.z (- (Transformation|GetWorldLocation (Variables|/Game/ThirdPersonBP/Blueprints/ThirdPersonCharacter.ThirdPersonCharacter_C|GetFollowCamera _asthird_person_character)) (Transformation|GetWorldLocation (Variables|Default|GetDefaultSceneRoot)))))) "0, 0, 0")) false false))

(event EventBeginPlay)

(event Collision|EventActorBeginOverlap
  (params (OtherActor :type Actor%20Object%20Reference)))

(event EventTick
  (params (DeltaSeconds :type Float%20%28single-precision%29))
  (if (Variables|Default|GetTextVis)
    (CallFunction|FacePlayer)))

(fn ConstructionScript)

(fn PickUpFunction)

(fn PuzzleFunction)

(fn LookforItem
  (params (name :type String))
  (LocalVariables|SetFound false)
  (bind _array_element (Utilities|Array|ForEachLoopwithBreak (Variables|/Game/ThirdPersonBP/Blueprints/ThirdPersonCharacter.ThirdPersonCharacter_C|GetItemList (Variables|Default|Getplayer)) :!label _label)
    (:LoopBody
      (if (Utilities|Enum|Equal(Enum) _array_element name)
        (LocalVariables|SetFound true)
        (goto _label Break)))
    (:Completed
      (return (LocalVariables|GetFound)))))