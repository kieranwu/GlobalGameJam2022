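; Lever is an interactable pickup actor that adds its item name to the player's item list.
; Each tick runs the parent logic, then calls the pickup function while TextVis is set and the player's PressE flag is true.
; The pickup function appends ItemName to the list, prints a confirmation and destroys the actor.
; Overlap handling is left to the parent class.
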(event EventBeginPlay
  (|CallParentFunction) ; This node is disabled and will not be called.\nDrag off pins to build functionality.
)

(event Collision|EventActorBeginOverlap
  (params (OtherActor :type Actor%20Object%20Reference))
  (|CallParentFunction OtherActor))

(event EventTick
  (params (DeltaSeconds :type Float%20%28single-precision%29))
  (|CallParentFunction DeltaSeconds)
  (if (Variables|Default|GetTextVis)
    (if (Variables|/Game/ThirdPersonBP/Blueprints/ThirdPersonCharacter.ThirdPersonCharacter_C|GetPressE (Variables|Default|Getplayer))
      (CallFunction|PickUpFunction))))

(fn ConstructionScript
  (|CallParentFunction))

(fn PickUpFunction
  (Utilities|Array|Add (Variables|/Game/ThirdPersonBP/Blueprints/ThirdPersonCharacter.ThirdPersonCharacter_C|GetItemList (Variables|Default|Getplayer)) (Variables|Default|GetItemName))
  (Development|PrintString "Item picked up")
  (Actor|DestroyActor))